(event `ShowMainMenu`
  (bind _returnvalue (`GameplayStatics.GetPlayerController` 0))
  ;[1 1 1] Show Main Menu
  (`/Engine/EditorBlueprintResources/StandardMacros.IsValid` (`self.MainMenuWB`)
    (:`Is Valid`
      _)
    (:`Is Not Valid`
      (bind _returnvalue_2 (`|CreateWidget` "/Game/TransfinityPlayerCharacter/MOBAFight/UI/MainMenu/MainMenu_WB.MainMenu_WB_C" _returnvalue))
      (set `self.MainMenuWB` _returnvalue_2)))
  (`UserWidget.AddToViewport` (`self.MainMenuWB`) 0)
  (set `PlayerController.bShowMouseCursor` true _returnvalue))

(event `LaunchLobby`
  ;[1 1 1] Keep EveryOne Go To Gameplay Map
  (`self.ShowLoadingScreen`)
  (`CreateSessionCallbackProxy.CreateSession` (`GameplayStatics.GetPlayerController` 0) (`self.MaxPlayers`) (`self.UserLAN`)
    (:`OnSuccess`
      (`GameplayStatics.OpenLevel` "LobbyMap" true "listen"))))

(event `ShowLoadingScreen`
  ;[1 1 1] Show Loading Screen
  (`/Engine/EditorBlueprintResources/StandardMacros.IsValid` (`self.ShowLoadingScreenWB`)
    (:`Is Valid`
      _)
    (:`Is Not Valid`
      (bind _returnvalue (`|CreateWidget` "/Game/TransfinityPlayerCharacter/MOBAFight/UI/LoadingScreen_WB.LoadingScreen_WB_C"))
      (set `self.ShowLoadingScreenWB` _returnvalue)))
  (`UserWidget.AddToViewport` (`self.ShowLoadingScreenWB`) 0))

(event `JoinServer`
  (params (SessionToJoin :type "BlueprintSessionResult Structure"))
  ;[1 1 1] Joint Game Sesion
  (`self.ShowLoadingScreen`)
  (`JoinSessionCallbackProxy.JoinSession` (`GameplayStatics.GetPlayerController` 0) SessionToJoin))

(event `SaveGameCheck`
  ;[1 1 1] Check for Save Game
  (bind _returnvalue (`GameplayStatics.DoesSaveGameExist` (`self.PlayerSettingSave`)))
  (if _returnvalue
    (`self.ShowMainMenu`)
    (set `self.CreatedSaveFile?` true)
    (else
      (`self.ShowOptionMenu`)
      (set `PlayerController.bShowMouseCursor` true (`GameplayStatics.GetPlayerController` 0)))))

(event `Open Character Select`
  ;[1 1 1] Handle Opening Character Select Screen
  (bind _asyour_earth_controller (cast `/Game/TransfinityPlayerCharacter/YourEarthMain/YourEarthController` (`GameplayStatics.GetPlayerController` 0)))
  (`/Game/TransfinityPlayerCharacter/YourEarthMain/YourEarthController.AddHeroSelectToViewport` _asyour_earth_controller (`self.ServerName`))
  (`/Game/TransfinityPlayerCharacter/YourEarthMain/YourEarthController.InitialSetup` _asyour_earth_controller)
  (`/Game/TransfinityPlayerCharacter/YourEarthMain/YourEarthController.UpdateControlledState` _asyour_earth_controller "NewEnumerator4")
  (`CreateSessionCallbackProxy.CreateSession` (`GameplayStatics.GetPlayerController` 0) (`self.MaxPlayers`) (`self.UserLAN`)))

(event `ShowOptionMenu`
  ;[1 1 1] Show Option Menu
  (`/Engine/EditorBlueprintResources/StandardMacros.IsValid` (`self.OptionMenuWB`)
    (:`Is Valid`
      _)
    (:`Is Not Valid`
      (bind _returnvalue (`|CreateWidget` "/Game/TransfinityPlayerCharacter/COBA_Demo/UI/COBA_CreateUsername.COBA_CreateUsername_C"))
      (set `self.OptionMenuWB` _returnvalue)))
  (`UserWidget.AddToViewport` (`self.OptionMenuWB`) 0)
  (if (not (`self.CreatedSaveFile?`))
    (set `/Game/TransfinityPlayerCharacter/COBA_Demo/UI/COBA_CreateUsername.WelcomeMessageVis` "Visible" (`self.OptionMenuWB`))))

(event `LoadCOBAMenu`
  ;[0 0 0] Work With Third Party Related.
  (bind _returnvalue (`GameplayStatics.DoesSaveGameExist` (`self.PlayerSettingSave`)))
  (if _returnvalue
    (`self.Open Character Select`)
    (else
      (`self.ShowOptionMenu`)
      (set `PlayerController.bShowMouseCursor` true (`GameplayStatics.GetPlayerController` 0)))))

(event `ValidateCharRef`
  ;[0 0 0] Your Earth Related
  (bind _asals_anim_man_character_bp (cast `/Game/TransfinityPlayerCharacter/AdvancedLocomotionV4/Blueprints/CharacterLogic/ALS_AnimMan_CharacterBP` (`GameplayStatics.GetPlayerCharacter` 0)))
  (set `self.PlayerTransformRef` (`SceneComponent.K2_GetComponentToWorld` (`Character.Mesh` _asals_anim_man_character_bp)))
  (`self.LoadCOBAMenu`))

(event `LoadBackIntoYourEarth`
  ;[0 0 0] Work With Third Party Related.
  (`GameplayStatics.OpenLevel` (`self.YourEarthMap`))
  (set `self.LoadPlayerTransform` true))