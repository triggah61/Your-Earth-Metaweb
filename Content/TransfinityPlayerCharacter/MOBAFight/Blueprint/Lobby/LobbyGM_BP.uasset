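; Lobby game mode for a MOBA-style game that tracks joining players and coordinates character, team and ready state before the match.
; PostLogin registers each controller on the server and sets up its lobby menu from game instance data.
; EveryOneUpdate rebuilds the player list, pushes lobby state to every LobbyPC_BP and calls their start events when all are ready.
; QuitUpdate removes leavers and refreshes; LuanchTheGame server-travels to the fixed TopDownGameMap.
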(event `self.K2_PostLogin`
  (params (NewPlayer :type "PlayerController Object Reference"))
  ;[1 1 1] **BEGIN   Add Player to Game and set array
  (`/Engine/EditorBlueprintResources/ActorMacros.Switch Has Authority`
    (:`Authority`
      (`KismetArrayLibrary.Array_Add` (`self.AllPlayerController`) NewPlayer)
      ;[1 1 1] Add Server Name and Max Player Infomation
      (bind _asmaster_game_instance_bp (cast `/Game/TransfinityPlayerCharacter/MOBAFight/Blueprint/AllLevel/MasterGameInstance_BP` (`GameplayStatics.GetGameInstance`)))
      (set `self.ServerName` (`/Game/TransfinityPlayerCharacter/MOBAFight/Blueprint/AllLevel/MasterGameInstance_BP.ServerName` _asmaster_game_instance_bp))
      (set `self.MaxPlayers` (`/Game/TransfinityPlayerCharacter/MOBAFight/Blueprint/AllLevel/MasterGameInstance_BP.MaxPlayers` _asmaster_game_instance_bp))
      ;[1 1 1] Create Lobby Menu and Initial Setup Data
      (bind _aslobby_pc_bp (cast `/Game/TransfinityPlayerCharacter/MOBAFight/Blueprint/Lobby/LobbyPC_BP` NewPlayer))
      (`/Game/TransfinityPlayerCharacter/MOBAFight/Blueprint/Lobby/LobbyPC_BP.SetupLobbyMenu` _aslobby_pc_bp (`self.ServerName`))
      (`/Game/TransfinityPlayerCharacter/MOBAFight/Blueprint/Lobby/LobbyPC_BP.InitialSetup` _aslobby_pc_bp))))

(event `EveryOneUpdate`
  (bind _allplayercontroller (`self.AllPlayerController`))
  ;[0.3589 0.3698 0.3616] ( Run from Server ) , Update Everything to all Client in Connect in the Game
  ;;[1 1 1] Comment
  (bind _output_get (set `self.CurrentPlayer` (`KismetArrayLibrary.Array_Length` (`self.AllPlayerController`))))
  (if (> _output_get 0)
    (`KismetArrayLibrary.Array_Clear` (`self.ConnectedPlayers`))
    (set `self.AllReady` true)
    (for _array_element _allplayercontroller
      (bind _aslobby_pc_bp (cast `/Game/TransfinityPlayerCharacter/MOBAFight/Blueprint/Lobby/LobbyPC_BP` _array_element))
      (`KismetArrayLibrary.Array_Add` (`self.ConnectedPlayers`) (`/Game/TransfinityPlayerCharacter/MOBAFight/Blueprint/Lobby/LobbyPC_BP.PlayerSettings` _aslobby_pc_bp))
      ;;[0.3589 0.3698 0.3616] Update Text in Widget Menu of Number of Player (format 9/9)
      (`/Game/TransfinityPlayerCharacter/MOBAFight/Blueprint/Lobby/LobbyPC_BP.UpdateNumberofPlayers` _aslobby_pc_bp (`self.CurrentPlayer`) (`self.MaxPlayers`)))
    (for _array_element_2 _allplayercontroller
      (bind _aslobby_pc_bp_2 (cast `/Game/TransfinityPlayerCharacter/MOBAFight/Blueprint/Lobby/LobbyPC_BP` _array_element_2))
      ;;[0.3589 0.3698 0.3616] Update List Name of Player Connection
      (`/Game/TransfinityPlayerCharacter/MOBAFight/Blueprint/Lobby/LobbyPC_BP.AddPlayerInfo` _aslobby_pc_bp_2 (`self.ConnectedPlayers`))
      ;;[0.3589 0.3698 0.3616] Update Avalilable Character can Chosse
      (`/Game/TransfinityPlayerCharacter/MOBAFight/Blueprint/Lobby/LobbyPC_BP.UpdateAvalilableCharacter` _aslobby_pc_bp_2 (`self.CharacterAvailable`))
      ;;[0.3589 0.3698 0.3616] Update Picture and Name in Bar Team
      (`/Game/TransfinityPlayerCharacter/MOBAFight/Blueprint/Lobby/LobbyPC_BP.UpdateShowTeam` _aslobby_pc_bp_2 (`self.BetaTeam`) (`self.AlphaTeam`)))
    (for _array_element_3 _allplayercontroller
      (bind _aslobby_pc_bp_3 (cast `/Game/TransfinityPlayerCharacter/MOBAFight/Blueprint/Lobby/LobbyPC_BP` _array_element_3))
      ;;[0.1667 0.1667 0.1667] Check All Client Ready To Play
      (`self.CheckAllReady` (`/Game/TransfinityPlayerCharacter/MOBAFight/Blueprint/Lobby/LobbyPC_BP.PlayerSettings` _aslobby_pc_bp_3)))
    (if (`self.AllReady`)
      (for _array_element_4 (`self.AllPlayerController`)
        (bind _aslobby_pc_bp_4 (cast `/Game/TransfinityPlayerCharacter/MOBAFight/Blueprint/Lobby/LobbyPC_BP` _array_element_4))
        (`/Game/TransfinityPlayerCharacter/MOBAFight/Blueprint/Lobby/LobbyPC_BP.CallStartEvent` _aslobby_pc_bp_4)))))

(event `LuanchTheGame`
  ;[0.3589 0.3698 0.3616] Launch the game based on map selection from Game Setting.
  (`KismetSystemLibrary.ExecuteConsoleCommand` "servertravel /Game/MOBAFight/Maps/TopDownGameMap" (`GameplayStatics.GetPlayerController` 0)))

(event `QuitUpdate`
  (params (PlayerController :type "PlayerController Object Reference"))
  ;[0.3589 0.3698 0.3616] Quit Session Update
  (for (_array_element _array_index) (`self.AllPlayerController`)
    (if (== _array_element PlayerController)
      (`KismetArrayLibrary.Array_Remove` (`self.AllPlayerController`) _array_index)
      (`self.EveryOneUpdate`))))

(fn `CheckAllReady`
  (params (PlayerInfo :type "/Game/TransfinityPlayerCharacter/MOBAFight/Structure/ST_PlayerInfo Structure"))
  (set `self.AllReady` (`KismetMathLibrary.Conv_IntToBool` (* (`KismetMathLibrary.Conv_BoolToInt` (`.MyReadyFlag_24_A1A7E0F0487076EB468011B343F3A4A6` (break `/Game/TransfinityPlayerCharacter/MOBAFight/Structure/ST_PlayerInfo` PlayerInfo))) (`KismetMathLibrary.Conv_BoolToInt` (`self.AllReady`))))))

(fn `InitialCharAvailable`
  (locals (Available :type Boolean :default true))
  (bind _characteravailable (`self.CharacterAvailable`))
  (`KismetArrayLibrary.Array_Clear` _characteravailable)
  (`KismetArrayLibrary.Array_Resize` _characteravailable (`KismetArrayLibrary.Array_Length` (`/Game/TransfinityPlayerCharacter/MOBAFight/Blueprint/AllLevel/MasterGameInstance_BP.CharacterDB` (cast `/Game/TransfinityPlayerCharacter/MOBAFight/Blueprint/AllLevel/MasterGameInstance_BP` (`GameplayStatics.GetGameInstance`) :!pure true))))
  (for (_ _array_index) (`self.CharacterAvailable`)
    (`KismetArrayLibrary.Array_Set` (`self.CharacterAvailable`) _array_index (`local.Available`))))

(fn `UserConstructionScript`)