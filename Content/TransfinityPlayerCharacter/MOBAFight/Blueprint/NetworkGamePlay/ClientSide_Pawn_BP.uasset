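; Client-side camera pawn for a MOBA game that pans the in-game view when the mouse is dragged.
; MoveDirection receives a direction code and controller reference, then offsets the pawn in X/Y along one of eight straight or diagonal directions at the controller's camera speed.
; Per-direction limit macros compare the current location against X/Y bounds to gate each new position before SetActorLocation applies it.
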(event `MoveDirection`
  (params (DirectionValue :type Integer) (ClientSideControllerRef :type "/Game/TransfinityPlayerCharacter/MOBAFight/Blueprint/NetworkGamePlay/ClientSide_Controller_BP Object Reference"))
  (bind _speedmovecamera (`/Game/TransfinityPlayerCharacter/MOBAFight/Blueprint/NetworkGamePlay/ClientSide_Controller_BP.SpeedMoveCamera` (`self.ClientSideControllerRef`)))
  (bind _speedmovecamera_2 (`/Game/TransfinityPlayerCharacter/MOBAFight/Blueprint/NetworkGamePlay/ClientSide_Controller_BP.SpeedMoveCamera` (`self.ClientSideControllerRef`)))
  (bind _speedmovecamera_3 (`/Game/TransfinityPlayerCharacter/MOBAFight/Blueprint/NetworkGamePlay/ClientSide_Controller_BP.SpeedMoveCamera` (`self.ClientSideControllerRef`)))
  (bind _speedmovecamera_4 (`/Game/TransfinityPlayerCharacter/MOBAFight/Blueprint/NetworkGamePlay/ClientSide_Controller_BP.SpeedMoveCamera` (`self.ClientSideControllerRef`)))
  ;[1 1 1] Process Move Camera In Game When Drag Mouse
  (set `self.ClientSideControllerRef` ClientSideControllerRef)
  (switch `int` DirectionValue
    (:`1`
      ;;[1 0 0.8571] ** Update Version 4.00 Limit Camera Move
      (if (<= (.x (`self.K2_GetActorLocation`)) (`self.Limit(+X)`))
        (set `self.PositionMove` (`KismetMathLibrary.MakeVector` (+ (.x (`self.K2_GetActorLocation`)) (`/Game/TransfinityPlayerCharacter/MOBAFight/Blueprint/NetworkGamePlay/ClientSide_Controller_BP.SpeedMoveCamera` (`self.ClientSideControllerRef`))) (.y (`self.K2_GetActorLocation`)) (.z (`self.K2_GetActorLocation`))))
        (`self.K2_SetActorLocation` self (`self.PositionMove`) false false :!label _label)))
    (:`2`
      (if (>= (.x (`self.K2_GetActorLocation`)) (`self.Limit(-X)`))
        (set `self.PositionMove` (`KismetMathLibrary.MakeVector` (- (.x (`self.K2_GetActorLocation`)) (`/Game/TransfinityPlayerCharacter/MOBAFight/Blueprint/NetworkGamePlay/ClientSide_Controller_BP.SpeedMoveCamera` (`self.ClientSideControllerRef`))) (.y (`self.K2_GetActorLocation`)) (.z (`self.K2_GetActorLocation`))))
        (goto _label)))
    (:`3`
      (if (>= (.y (`self.K2_GetActorLocation`)) (`self.Limit(-Y)`))
        (set `self.PositionMove` (`KismetMathLibrary.MakeVector` (.x (`self.K2_GetActorLocation`)) (- (.y (`self.K2_GetActorLocation`)) (`/Game/TransfinityPlayerCharacter/MOBAFight/Blueprint/NetworkGamePlay/ClientSide_Controller_BP.SpeedMoveCamera` (`self.ClientSideControllerRef`))) (.z (`self.K2_GetActorLocation`))))
        (goto _label)))
    (:`4`
      (if (<= (.y (`self.K2_GetActorLocation`)) (`self.Limit(+Y)`))
        (set `self.PositionMove` (`KismetMathLibrary.MakeVector` (.x (`self.K2_GetActorLocation`)) (+ (.y (`self.K2_GetActorLocation`)) (`/Game/TransfinityPlayerCharacter/MOBAFight/Blueprint/NetworkGamePlay/ClientSide_Controller_BP.SpeedMoveCamera` (`self.ClientSideControllerRef`))) (.z (`self.K2_GetActorLocation`))))
        (goto _label)))
    (:`5`
      (if (and (<= (.x (`self.K2_GetActorLocation`)) (`self.Limit(+X)`)) (>= (.y (`self.K2_GetActorLocation`)) (`self.Limit(-Y)`)))
        (set `self.PositionMove` (`KismetMathLibrary.MakeVector` (+ (.x (`self.K2_GetActorLocation`)) _speedmovecamera) (- (.y (`self.K2_GetActorLocation`)) _speedmovecamera) (.z (`self.K2_GetActorLocation`))))
        (goto _label)))
    (:`6`
      (if (and (<= (.x (`self.K2_GetActorLocation`)) (`self.Limit(+X)`)) (<= (.y (`self.K2_GetActorLocation`)) (`self.Limit(+Y)`)))
        (set `self.PositionMove` (`KismetMathLibrary.MakeVector` (+ (.x (`self.K2_GetActorLocation`)) _speedmovecamera_2) (+ (.y (`self.K2_GetActorLocation`)) _speedmovecamera_2) (.z (`self.K2_GetActorLocation`))))
        (goto _label)))
    (:`7`
      (if (and (>= (.x (`self.K2_GetActorLocation`)) (`self.Limit(-X)`)) (>= (.y (`self.K2_GetActorLocation`)) (`self.Limit(-Y)`)))
        (set `self.PositionMove` (`KismetMathLibrary.MakeVector` (- (.x (`self.K2_GetActorLocation`)) _speedmovecamera_3) (- (.y (`self.K2_GetActorLocation`)) _speedmovecamera_3) (.z (`self.K2_GetActorLocation`))))
        (goto _label)))
    (:`8`
      (if (and (>= (.x (`self.K2_GetActorLocation`)) (`self.Limit(-X)`)) (<= (.y (`self.K2_GetActorLocation`)) (`self.Limit(+Y)`)))
        (set `self.PositionMove` (`KismetMathLibrary.MakeVector` (- (.x (`self.K2_GetActorLocation`)) _speedmovecamera_4) (+ (.y (`self.K2_GetActorLocation`)) _speedmovecamera_4) (.z (`self.K2_GetActorLocation`))))
        (goto _label)))))

(fn `UserConstructionScript`)